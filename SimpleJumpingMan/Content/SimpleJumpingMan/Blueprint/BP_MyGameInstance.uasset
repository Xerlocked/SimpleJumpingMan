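; BP_MyGameInstance is the game instance for SimpleJumpingMan that tracks how many coins remain.
; SetupCoinCount sets RemainCoin from the number of BP_Coin actors found in the world.
; DecreamentCoin lowers that count and runs CheckRemainCoin, which fires the OnClearCoin dispatcher once none are left.
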(fn CheckRemainCoin
  (if (<= (Variables|Default|GetRemainCoin) 0)
    (Default|CallOnClearCoin)))

(fn SetupCoinCount
  (bind _outactors (Actor|GetAllActorsOfClass "/Game/SimpleJumpingMan/Blueprint/BP_Coin.BP_Coin_C"))
  (Variables|Default|SetRemainCoin (Utilities|Array|Length _outactors)))

(fn DecreamentCoin
  (Math|Integer|DecrementInt (Variables|Default|GetRemainCoin)
    (:%20%20
      (CallFunction|CheckRemainCoin))))